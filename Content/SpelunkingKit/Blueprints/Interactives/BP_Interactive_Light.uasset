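; Interactive light for the spelunking kit that toggles a point light, particles, audio and prompt text on LightInteract.
; BeginPlay inverts InitiallyLit and runs the same toggle to apply the starting state.
; A timeline eases the mesh's "FireGlow" material parameter, using a dynamic instance and defaults cached in the construction script.
; A flicker timeline varies light intensity and position for moving shadows, but nothing in the graph triggers it.
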(event Custom|LightInteract
  ;[0 0 0] Light interaction
  ;;[1 1 1] Check if currently on or off
  (if (Variables|Default|GetOn/Off)
    ;;[1 1 1] Set on/off state of light and change prompt text
    (Variables|Default|SetOn/Off false)
    (Variables|Default|SetPromptText (Variables|Default|GetPromptText_Alternative))
    ;;[1 1 1] Enable/Disable light
    (Rendering|SetVisibility (Variables|Default|GetPointLight) false false)
    (Components|Activation|Deactivate (Variables|Default|GetParticleSystem))
    ;;[1 1 1] Play material glow animation
    (CallFunction|Reverse)
    (else
      (Variables|Default|SetOn/Off true)
      (Variables|Default|SetPromptText (Variables|Default|GetPromptText_Default))
      (Rendering|SetVisibility (Variables|Default|GetPointLight) true false)
      (Components|Activation|Activate (Variables|Default|GetParticleSystem) false)
      (CallFunction|Play))))

(event Custom|Play
  ;[0 0 0] Material emissive animation (This fades in/out the orange glow if the material has named parameter)
  ;;[1 1 1] Animation timeline
  (bind _emissivealpha (Timeline|LightGlowAnimation Play)
    (:Update
      ;;[1 1 1] Set material instance parameter value
      (Rendering|Material|SetScalarParameterValue (Variables|Default|GetMaterialInstance) "FireGlow" (Class|KismetMathLibrary|FInterpEaseinOut (Variables|Default|GetCurrentGlowValue) (Variables|Default|GetDefaultGlowValue) _emissivealpha 2.0) :!class /Script/Engine.MaterialInstanceDynamic))))

(event Custom|Reverse
  ;[0 0 0] Material emissive animation (This fades in/out the orange glow if the material has named parameter)
  ;;[1 1 1] Animation timeline
  (bind _emissivealpha (Timeline|LightGlowAnimation Reverse)
    (:Update
      ;;[1 1 1] Set material instance parameter value
      (Rendering|Material|SetScalarParameterValue (Variables|Default|GetMaterialInstance) "FireGlow" (Class|KismetMathLibrary|FInterpEaseinOut (Variables|Default|GetCurrentGlowValue) (Variables|Default|GetDefaultGlowValue) _emissivealpha 2.0) :!class /Script/Engine.MaterialInstanceDynamic))))

(event EventBeginPlay
  ;[0 0 0] Light interaction
  ;;[1 1 1] Set initial lit state, set to opposite on/off and run the interact event to flip light on/off on begin play
  (if (Variables|Default|GetInitiallyLit)
    (Variables|Default|SetOn/Off false)
    (else
      (Variables|Default|SetOn/Off true)))
  ;;[1 1 1] Check if currently on or off
  (if (Variables|Default|GetOn/Off)
    ;;[1 1 1] Set on/off state of light and change prompt text
    (Variables|Default|SetOn/Off false)
    (Variables|Default|SetPromptText (Variables|Default|GetPromptText_Alternative))
    ;;[1 1 1] Enable/Disable light
    (Rendering|SetVisibility (Variables|Default|GetPointLight) false false)
    (Components|Activation|Deactivate (Variables|Default|GetParticleSystem))
    ;;[1 1 1] Play material glow animation
    (CallFunction|Reverse)
    (else
      (Variables|Default|SetOn/Off true)
      (Variables|Default|SetPromptText (Variables|Default|GetPromptText_Default))
      (Rendering|SetVisibility (Variables|Default|GetPointLight) true false)
      (Components|Activation|Activate (Variables|Default|GetParticleSystem) false)
      (CallFunction|Play))))

(fn ConstructionScript
  (|CallParentFunction)
  (Utilities|FlowControl|Sequence
    (:then_0
      ;[0 0 0] Interactive light construction script
      ;;[1 1 1] Store default light intensity
      (Variables|Default|SetDefaultLightIntensity (Variables|/Script/Engine.LightComponentBase|GetIntensity (Variables|Default|GetPointLight)))
      ;;[1 1 1] Store default light location
      (Variables|Default|SetDefaultLightLocation (Transformation|GetWorldLocation (Variables|Default|GetPointLight)))
      ;;[1 1 1] Set prompt text based on current state
      (Variables|Default|SetPromptText_Default (Variables|Default|GetPromptText))
      (if (Variables|Default|GetOn/Off)
        (Variables|Default|SetPromptText (Variables|Default|GetPromptText_Default))
        (else
          (Variables|Default|SetPromptText (Variables|Default|GetPromptText_Alternative)))))
    (:then_1
      ;[0 0 0] Set light glow material settings
      ;;[1 1 1] Create material instance from static mesh
      (bind _returnvalue (Rendering|Material|CreateDynamicMaterialInstance (Variables|Default|GetStaticMesh) 0 0 :!class /Script/Engine.PrimitiveComponent))
      (bind _output_get (Variables|Default|SetMaterialInstance _returnvalue))
      ;;[1 1 1] Store default glow value
      (bind _returnvalue_2 (Rendering|Material|GetScalarParameterValue _output_get "FireGlow" :!class /Script/Engine.MaterialInstanceDynamic))
      (Variables|Default|SetDefaultGlowValue _returnvalue_2)
      ;;[1 1 1] Set fire glow based on whether light is on/off
      (if (Variables|Default|GetInitiallyLit)
        (Rendering|Material|SetScalarParameterValue (Variables|Default|GetMaterialInstance) "FireGlow" (Variables|Default|GetDefaultGlowValue) :!class /Script/Engine.MaterialInstanceDynamic)
        (else
          (Rendering|Material|SetScalarParameterValue (Variables|Default|GetMaterialInstance) "FireGlow" 0.0 :!class /Script/Engine.MaterialInstanceDynamic))))))