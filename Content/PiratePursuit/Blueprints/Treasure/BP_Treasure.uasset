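; BP_Treasure is the treasure pickup Blueprint in PiratePursuit, driven entirely by actor overlap.
; An overlapping actor with a TreasureHolderComponent that is not in cooldown picks up the treasure, triggering a 2D coin sound and activating every BP_Water actor.
; When an actor without that component overlaps and is BP_Water, the treasure's TreasureRespawn component respawns it.
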(event Collision|EventActorBeginOverlap
  (params (OtherActor :type Actor%20Object%20Reference))
  (bind _returnvalue (Actor|GetComponentbyClass OtherActor "/Script/PiratePursuit.TreasureHolderComponent"))
  ;[1 1 1] Player collision
  (Utilities|IsValid _returnvalue
    (:Is%20Valid
      (if (not (Class|TreasureHolderComponent|InCooldownState _returnvalue))
        (Class|TreasureHolderComponent|PickupTreasure _returnvalue self)
        (Audio|PlaySound2D "/Game/PiratePursuit/Audio/coin.coin" 1.0 1.0 0.0 0 0)
        (bind _outactors (Actor|GetAllActorsOfClass "/Game/PiratePursuit/Blueprints/BP_Water.BP_Water_C"))
        (for _array_element _outactors
          (bind _aswater (Utilities|Casting|CastToWater _array_element))
          (Variables|/Script/PiratePursuit.Water|Setm_IsActive _aswater true))))
    (:Is%20Not%20Valid
      ;[1 1 1] Water collision
      (Utilities|Casting|CastToBP_Water OtherActor)
      (Class|TreasureRespawnComponent|Respawn (Variables|Default|GetTreasureRespawn)))))

(fn ConstructionScript)