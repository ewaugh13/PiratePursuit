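; PunchHitbox is a punch hit-detection actor that stuns and knocks back pirate characters it overlaps.
; It ignores the actor it is attached to and any pirate already stunned or in a stun grace period.
; On a valid hit it calls Stun on the victim's PlayerStunComponent, then adds a CharacterMovement force along the hitbox's forward vector, using heavily scaled-up KnockbackPower.
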(event Collision|EventActorBeginOverlap
  (params (OtherActor :type Actor%20Object%20Reference))
  (if (not (== OtherActor (Actor|GetAttachParentActor)))
    (bind _asbp_pirate_character (Utilities|Casting|CastToBP_PirateCharacter OtherActor))
    (if (not (or (Variables|/Game/PiratePursuit/Blueprints/Combat/PlayerStunComponent.PlayerStunComponent_C|GetIs%20Stunned (Variables|/Game/PiratePursuit/Blueprints/BP_PirateCharacter.BP_PirateCharacter_C|GetPlayerStunComponent _asbp_pirate_character)) (Variables|/Game/PiratePursuit/Blueprints/Combat/PlayerStunComponent.PlayerStunComponent_C|GetIs%20In%20Grace%20Period (Variables|/Game/PiratePursuit/Blueprints/BP_PirateCharacter.BP_PirateCharacter_C|GetPlayerStunComponent _asbp_pirate_character))))
      (Default|Stun (Variables|/Game/PiratePursuit/Blueprints/BP_PirateCharacter.BP_PirateCharacter_C|GetPlayerStunComponent _asbp_pirate_character))
      (Physics|AddForce (Variables|/Script/Engine.Character|GetCharacterMovement _asbp_pirate_character) (* (Transformation|GetActorForwardVector) (* (Variables|Default|GetKnockback%20Power) 1e+08))))))

(fn ConstructionScript)