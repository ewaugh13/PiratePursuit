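; Actor component that lets the player be stunned in combat, with a grace period afterwards that blocks repeat stuns.
; Stun zeroes the owner's CharacterMovement MaxWalkSpeed, then a timer restores the saved speed and starts the timed grace period.
; The punch sound plays on every Stun call, even when the stun itself is ignored.
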(event Custom|Stun
  (bind _returnvalue (Components|GetOwner))
  (bind _returnvalue_2 (Actor|GetComponentbyClass _returnvalue "/Script/Engine.CharacterMovementComponent"))
  ;[1 1 1] Stun
  (Audio|PlaySound2D "/Game/PiratePursuit/Audio/punch.punch" 1.0 1.0 0.0 0 0)
  (if (not (or (Variables|Default|GetIs%20Stunned) (Variables|Default|GetIs%20In%20Grace%20Period)))
    (Variables|Default|SetOriginal%20Max%20Speed (Variables|/Script/Engine.CharacterMovementComponent|GetMaxWalkSpeed _returnvalue_2))
    (Variables|/Script/Engine.CharacterMovementComponent|SetMaxWalkSpeed _returnvalue_2 0.0)
    (Variables|Default|SetIs%20Stunned true)
    (Utilities|Time|SetTimerbyEvent (delegate Custom|Unstun) (Variables|Default|GetStun%20Time))))

(event Custom|Start%20Grace%20Period
  ;[1 1 1] Grace Period
  (Variables|Default|SetIs%20In%20Grace%20Period true)
  (Utilities|Time|SetTimerbyEvent (delegate Custom|End%20Grace%20Period) (Variables|Default|GetGrace%20Period)))

(event Custom|End%20Grace%20Period
  ;[1 1 1] Grace Period
  (Variables|Default|SetIs%20In%20Grace%20Period false))

(event Custom|Unstun
  ;[1 1 1] Unstun
  (Variables|/Script/Engine.CharacterMovementComponent|SetMaxWalkSpeed (Actor|GetComponentbyClass (Components|GetOwner) "/Script/Engine.CharacterMovementComponent") (Variables|Default|GetOriginal%20Max%20Speed))
  (Variables|Default|SetIs%20Stunned false)
  (CallFunction|StartGracePeriod))