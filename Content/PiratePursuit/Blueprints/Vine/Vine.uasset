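; Swingable vine that a pirate character can grab, provided they can grapple and are not carrying treasure.
; Overlapping its sphere flags the pirate as hit; Tick then attaches them by snapping their movement primitive to the sphere each frame.
; While the pirate moves in air, forward force on the sphere drives the swing.
; Ending the overlap clears the hit flag and launches an attached pirate forward and upward, detaching them.
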(event OnComponentBeginOverlap(Sphere)
  (params (OverlappedComponent :type Primitive%20Component%20Object%20Reference) (OtherActor :type Actor%20Object%20Reference) (OtherComp :type Primitive%20Component%20Object%20Reference) (OtherBodyIndex :type Integer) (bFromSweep :type Boolean) (SweepResult :type Hit%20Result%20Structure%20%28by%20ref%29))
  (bind _asbp_pirate_character (Utilities|Casting|CastToBP_PirateCharacter OtherActor))
  (Variables|/Game/PiratePursuit/Blueprints/BP_PirateCharacter.BP_PirateCharacter_C|SetPlayerHit _asbp_pirate_character true))

(event OnComponentEndOverlap(Sphere)
  (params (OverlappedComponent :type Primitive%20Component%20Object%20Reference) (OtherActor :type Actor%20Object%20Reference) (OtherComp :type Primitive%20Component%20Object%20Reference) (OtherBodyIndex :type Integer))
  (bind _asbp_pirate_character (Utilities|Casting|CastToBP_PirateCharacter OtherActor))
  (Variables|/Game/PiratePursuit/Blueprints/BP_PirateCharacter.BP_PirateCharacter_C|SetPlayerHit _asbp_pirate_character false)
  (if (Variables|/Game/PiratePursuit/Blueprints/BP_PirateCharacter.BP_PirateCharacter_C|GetAttached _asbp_pirate_character)
    (Character|LaunchCharacter _asbp_pirate_character (+ (* (Transformation|GetActorForwardVector _asbp_pirate_character) 1.5e+03) (* (Transformation|GetActorUpVector _asbp_pirate_character) 1e+03)) true true)
    (Variables|/Game/PiratePursuit/Blueprints/BP_PirateCharacter.BP_PirateCharacter_C|SetAttached _asbp_pirate_character false)))

(event EventTick
  (params (DeltaSeconds :type Float%20%28single-precision%29))
  (Utilities|IsValid (stale OnComponentBeginOverlap(Sphere) _asbp_pirate_character)
    (:Is%20Valid
      (if (not (Variables|/Game/PiratePursuit/Blueprints/BP_PirateCharacter.BP_PirateCharacter_C|GetHasTreasure (stale OnComponentBeginOverlap(Sphere) _asbp_pirate_character)))
        (if (Variables|/Game/PiratePursuit/Blueprints/BP_PirateCharacter.BP_PirateCharacter_C|GetCanGrapple (stale OnComponentBeginOverlap(Sphere) _asbp_pirate_character))
          (if (Variables|/Game/PiratePursuit/Blueprints/BP_PirateCharacter.BP_PirateCharacter_C|GetPlayerHit (stale OnComponentBeginOverlap(Sphere) _asbp_pirate_character))
            (Variables|/Game/PiratePursuit/Blueprints/BP_PirateCharacter.BP_PirateCharacter_C|SetAttached (stale OnComponentBeginOverlap(Sphere) _asbp_pirate_character) true)
            (if (Variables|/Game/PiratePursuit/Blueprints/BP_PirateCharacter.BP_PirateCharacter_C|GetAttached (stale OnComponentBeginOverlap(Sphere) _asbp_pirate_character))
              (Transformation|SetWorldLocation (Variables|/Script/Engine.MovementComponent|GetUpdatedPrimitive (Variables|/Script/Engine.Character|GetCharacterMovement (stale OnComponentBeginOverlap(Sphere) _asbp_pirate_character))) (Transformation|GetWorldLocation (Variables|Default|GetSphere)) false false)
              (if (Variables|/Game/PiratePursuit/Blueprints/BP_PirateCharacter.BP_PirateCharacter_C|GetMoveInAir (stale OnComponentBeginOverlap(Sphere) _asbp_pirate_character))
                (Physics|AddForce (Variables|Default|GetSphere) (* (Transformation|GetActorForwardVector (stale OnComponentBeginOverlap(Sphere) _asbp_pirate_character)) 3e+04) "None" false)))))))))

(fn ConstructionScript)