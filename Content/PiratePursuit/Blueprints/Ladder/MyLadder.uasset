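; MyLadder is a climbable ladder actor for pirate characters, driven by overlaps on its collision box.
; When a BP_PirateCharacter without treasure enters the box, it switches to Flying movement and its Climb flag is set.
; Leaving the box always restores Walking and clears Climb, so treasure carriers cannot start climbing from an overlap.
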(event OnComponentBeginOverlap(CollisionBox)
  (params (OverlappedComponent :type Primitive%20Component%20Object%20Reference) (OtherActor :type Actor%20Object%20Reference) (OtherComp :type Primitive%20Component%20Object%20Reference) (OtherBodyIndex :type Integer) (bFromSweep :type Boolean) (SweepResult :type Hit%20Result%20Structure%20%28by%20ref%29))
  (bind _asbp_pirate_character (Utilities|Casting|CastToBP_PirateCharacter OtherActor))
  (if (not (Variables|/Game/PiratePursuit/Blueprints/BP_PirateCharacter.BP_PirateCharacter_C|GetHasTreasure _asbp_pirate_character))
    (Pawn|Components|CharacterMovement|SetMovementMode (Variables|/Script/Engine.Character|GetCharacterMovement _asbp_pirate_character) "MOVE_Flying" 0)
    (Variables|/Game/PiratePursuit/Blueprints/BP_PirateCharacter.BP_PirateCharacter_C|SetClimb _asbp_pirate_character true)))

(event OnComponentEndOverlap(CollisionBox)
  (params (OverlappedComponent :type Primitive%20Component%20Object%20Reference) (OtherActor :type Actor%20Object%20Reference) (OtherComp :type Primitive%20Component%20Object%20Reference) (OtherBodyIndex :type Integer))
  (bind _asbp_pirate_character (Utilities|Casting|CastToBP_PirateCharacter OtherActor))
  (Pawn|Components|CharacterMovement|SetMovementMode (Variables|/Script/Engine.Character|GetCharacterMovement _asbp_pirate_character) "MOVE_Walking" 0)
  (Variables|/Game/PiratePursuit/Blueprints/BP_PirateCharacter.BP_PirateCharacter_C|SetClimb _asbp_pirate_character false))

(event EventBeginPlay)

(event Collision|EventActorBeginOverlap
  (params (OtherActor :type Actor%20Object%20Reference)))

(event EventTick
  (params (DeltaSeconds :type Float%20%28single-precision%29)))

(fn ConstructionScript)